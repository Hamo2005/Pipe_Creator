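; BP_Pipe is a pipe actor that renders a spline as a chain of spline meshes and adjusts its point count as its end changes length.
; Every Tick destroys and recreates the meshes from world-space point locations and tangents, without clearing their array or attaching them (attach node is unwired).
; It then duplicates the last point when the final segment exceeds MaxDistance, or removes it when it falls within MaxDistance of the third-last.
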(event Custom|Update%20Spline%20Points%20Num
  (bind _spline (Variables|Default|GetSpline))
  (bind _spline_2 (Variables|Default|GetSpline))
  (bind _max_distance (Variables|Data|GetMax%20Distance))
  (bind _returnvalue (Spline|GetNumberOfSplinePoints _spline))
  (bind _returnvalue_2 (- _returnvalue 1))
  (bind _returnvalue_3 (Spline|GetLocationatSplinePoint _spline _returnvalue_2 "World"))
  ;[1 1 1] Update Spline Points Num
  (Utilities|FlowControl|Sequence
    (:then_0
      (if (> (Math|Vector|Distance(Vector) (Spline|GetLocationatSplinePoint _spline (- _returnvalue 2) "World") _returnvalue_3) _max_distance)
        (Spline|AddSplinePoint _spline_2 _returnvalue_3 "World" true)))
    (:then_1
      (if (< (Math|Vector|Distance(Vector) _returnvalue_3 (Spline|GetLocationatSplinePoint _spline (- _returnvalue 3) "World")) _max_distance)
        (if (> _returnvalue_2 1)
          (Spline|RemoveSplinePoint _spline_2 _returnvalue_2 true))))))

(event EventTick
  (params (DeltaSeconds :type Float%20%28single-precision%29))
  ;[1 1 1] Update
  (Utilities|FlowControl|Sequence
    (:then_0
      (Pipe|UpdateSplineMeshes))
    (:then_1
      (CallFunction|UpdateSplinePointsNum))))

(fn ConstructionScript)

(fn UpdateSplineMeshes
  (bind _spline (Variables|Default|GetSpline))
  ;[1 1 1] Update Spline Meshes
  (for _array_element (Variables|SplinePoints|GetSpline%20Meshes)
    (Utilities|IsValid _array_element
      (:Is%20Valid
        (Components|DestroyComponent _array_element))))
  (for _index (range 0 (- (Spline|GetNumberOfSplinePoints _spline) 1))
    (bind _returnvalue (AddComponent|AddSplineMeshComponent true))
    (Utilities|IsValid _returnvalue
      (:Is%20Valid
        (Utilities|Array|Add (Variables|SplinePoints|GetSpline%20Meshes) _returnvalue)
        (Utilities|FlowControl|Sequence
          (:then_0
            (Components|StaticMesh|SetStaticMesh _returnvalue (Variables|Data|GetPipe%20Mesh)))
          (:then_1
            (SplineMesh|SetForwardAxis _returnvalue (Variables|Data|GetPipe%20Forward%20Axis) true))
          (:then_3
            ;;[1 1 1] Set Start & End
            (SplineMesh|SetStartandEnd _returnvalue (Spline|GetLocationatSplinePoint _spline _index "World") (Spline|GetTangentatSplinePoint _spline _index "World") (Spline|GetLocationatSplinePoint _spline (+ _index 1) "World") (Spline|GetTangentatSplinePoint _spline (+ _index 1) "World") true :!class /Script/Engine.SplineMeshComponent)))))))

(fn BaseData
  (return (Transformation|GetActorLocation) (Transformation|GetActorRotation)))

(fn PipeData
  (return (Variables|Data|GetPipe%20Mesh) (Variables|Data|GetPipe%20Forward%20Axis) 0.0))

(fn SplineData
  (bind _spline (Variables|Default|GetSpline))
  (bind _returnvalue (Spline|GetNumberOfSplinePoints _spline))
  (return _returnvalue (- _returnvalue 1)))