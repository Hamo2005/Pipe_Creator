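; BP_Connector is an actor that acts as an attachment point for BP_Pipe actors and tracks its link to another connector.
; It spawns a cylinder-mesh pipe at its PipeLocation component and can destroy it.
; Set and reset events assign or clear the pipe, connected connector and state flags.
; Getter functions expose its transform, forward axis and pipe state, while an attach-to-mesh call sits unconnected.
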(event Custom|Spawn%20Pipe
  (bind _pipe_location (Variables|Default|GetPipe%20Location))
  (bind _returnvalue (Transformation|GetWorldTransform _pipe_location))
  ;[1 1 1] Spawn Pipe
  (bind _returnvalue_2 (Game|SpawnActorfromClass "/Game/Blueprints/Actors/BP_Pipe.BP_Pipe_C" (Math|Transform|MakeTransform (.location _returnvalue) (.rotation _returnvalue)) "Undefined" 0 "/Game/Demo_Content/Assets/SM_Cylinder.SM_Cylinder" "Z" 0))
  (bind _output_get (Variables|Ref|SetCurrent%20Pipe _returnvalue_2))
  (Variables|PipeCreator|SetHas%20Pipe true))

(event Custom|Destroy%20Pipe
  ;[1 1 1] Destroy Pipe
  (Variables|PipeCreator|SetHas%20Pipe false)
  (bind _current_pipe (Variables|Ref|GetCurrent%20Pipe)
    (:then
      (Actor|DestroyActor _current_pipe))
    (:else)))

(event Custom|Set%20New%20Pipe
  (params (Current%20Pipe :type BP%20Pipe%20Object%20Reference) (Connected%20Connector :type BP%20Connector%20Object%20Reference) (Is%20other%20Connector :type Boolean))
  ;[1 1 1] Set New Pipe
  (Utilities|FlowControl|Sequence
    (:then_0
      (Utilities|IsValid Current%20Pipe
        (:Is%20Valid
          (Variables|Ref|SetCurrent%20Pipe Current%20Pipe))))
    (:then_1
      (Variables|PipeCreator|SetHas%20Pipe true)
      (Variables|Default|SetIs%20other%20Connector Is%20other%20Connector))
    (:then_2
      (Utilities|IsValid Connected%20Connector
        (:Is%20Valid
          (Variables|Default|SetConnected%20Connector Connected%20Connector))))))

(event Custom|Reset%20New%20Pipe
  ;[1 1 1] Reset New Pipe
  (Utilities|FlowControl|Sequence
    (:then_0
      (Variables|Ref|SetCurrent%20Pipe 0))
    (:then_1
      (Variables|PipeCreator|SetHas%20Pipe false)
      (Variables|Default|SetIs%20other%20Connector false)
      (Development|PrintString "......."))
    (:then_2
      (Variables|Default|SetConnected%20Connector 0))))

(fn ConstructionScript)

(fn BaseData
  (return (Transformation|GetActorLocation) (Transformation|GetActorRotation)))

(fn ConnectorData
  (return (Variables|Data|GetForward%20Axis)))

(fn PipeData
  (return (Variables|Ref|GetCurrent%20Pipe) (Variables|Default|GetConnected%20Connector) (Variables|Default|GetPipe%20Location) (Variables|PipeCreator|GetHas%20Pipe) (Variables|Default|GetIs%20other%20Connector)))